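; Mutant enemy that roams, chases a sighted player and performs melee attacks, with an overhead health bar shown when the player is near.
; A BehaviorUnit state machine uses AI MoveTo to alternate random wandering with nearest patrol points, switching to chase through PawnSensing.
; A DoOnce-gated montage triggers a sphere-trace damage check via notify, then resets.
; SetDamage subtracts fixed health; death leads to delayed destruction and a game-mode save.
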(event `self.ReceiveBeginPlay`
  (bind _aswbp_health_bar_enemy (cast `/Game/ProjectHooks/Blueprints/Mutant/WBP_HealthBarEnemy` (`WidgetComponent.GetUserWidgetObject` (`self.HealthBar`))))
  (bind _output_get (set `self.HealthWidgetRef` _aswbp_health_bar_enemy))
  (set `/Game/ProjectHooks/Blueprints/Mutant/WBP_HealthBarEnemy.Health` (`self.Health`) _output_get)
  (set `/Game/ProjectHooks/Blueprints/Mutant/WBP_HealthBarEnemy.HealthMax` (`self.HealthMax`) _output_get)
  (`self.BehaviorUnit`))

(event `BehaviorUnit`
  (bind _charactermovement (`self.CharacterMovement`))
  ;[1 0.02367 0] AI Behavior Logic
  (if (not (`self.Dead?`))
    (switch `/Game/ProjectHooks/Blueprints/Mutant/BehaviorModes` (`self.BehaviorModes`)
      (:`NewEnumerator0`
        ;;[0 0.3175 1] Roam1
        (`|AIMoveTo` self (`NavigationSystemV1.K2_GetRandomReachablePointInRadius` (`self.K2_GetActorLocation`) (`self.RoamRadius`) null null) null
          (:`OnSuccess`
            (`self.UpdatePatrolPoint`)
            (`KismetSystemLibrary.Delay` (`KismetMathLibrary.RandomFloatInRange` (`self.MinWait`) (`self.MaxWait`)))
            (if (`|EnumEquality` (`self.BehaviorModes`) "NewEnumerator2")
              (`self.ChasePlayer`)
              (else
                (set `self.BehaviorModes` "NewEnumerator1")
                (`self.BehaviorUnit`))))))
      (:`NewEnumerator1`
        ;;[1 0.6174 0] Roam2
        (`|AIMoveTo` self (0.0 0.0 0.0) (`self.PatrolPointRef`)
          (:`OnSuccess`
            (`KismetSystemLibrary.Delay` (`KismetMathLibrary.RandomFloatInRange` (`self.MinWait`) (`self.MaxWait`)))
            (if (`|EnumEquality` (`self.BehaviorModes`) "NewEnumerator2")
              (`self.ChasePlayer`)
              (else
                (set `self.BehaviorModes` "NewEnumerator0")
                (`self.BehaviorUnit`))))))
      (:`NewEnumerator2`
        ;;[1 0 0.8591] Chase Player
        (if (not (`self.Dead?`)) :!label _label
          (`|AIMoveTo` self (0.0 0.0 0.0) (`self.AttackTarget`) (`self.AttackAcceptanceRadius`)
            (:`OnSuccess`
              (if (not (`self.Dead?`))
                (`/Engine/EditorBlueprintResources/StandardMacros.DoOnce` false :!label _label_2
                  (:`Completed`
                    (set `self.AttackingPlayer?` false)
                    (bind _notifyname (`|PlayMontage` (`self.Mesh`) (`self.AttackMontage`))
                      (:`then`
                        (`MovementComponent.StopMovementImmediately` _charactermovement)
                        (set `CharacterMovementComponent.MaxWalkSpeed` 0.0 _charactermovement)
                        (`self.TrackPlayer`))
                      (:`OnCompleted`
                        (`KismetSystemLibrary.Delay` (`KismetMathLibrary.RandomFloatInRange` 0.1 0.3))
                        (set `self.AttackingPlayer?` false)
                        (if (not (`self.Dead?`))
                          (`self.ReleaseAttack`)
                          (set `CharacterMovementComponent.MaxWalkSpeed` 450.0 (`self.CharacterMovement`))
                          (`self.BehaviorUnit`)))
                      (:`OnNotifyBegin`
                        (switch `name` _notifyname
                          (:`AttackTrace`
                            (`self.AttackTrace`)))))))))))))))

(event `ChasePlayer`
  ;[1 0.02367 0] AI Behavior Logic
  ;;[1 0 0.8591] Chase Player
  (goto _label))

(event `ReleaseAttack`
  ;[1 0.02367 0] AI Behavior Logic
  ;;[1 0 0.8591] Chase Player
  (goto _label_2 :!via `Reset`))

(event `self.PawnSensing.OnSeePawn`
  (params (Pawn :type "Pawn Object Reference"))
  ;[0 1 0.06933] See Player?
  (if (not (`self.Dead?`))
    (bind _asbp_player_character (cast `/Game/FlexibleCombatSystem/Blueprints/BP_PlayerCharacter` Pawn))
    (set `self.AttackTarget` _asbp_player_character)
    (set `self.BehaviorModes` "NewEnumerator2")
    (`self.BehaviorUnit`)))

(event `TrackPlayer`
  (bind (_returnvalue_roll _returnvalue_pitch _returnvalue_yaw) (`KismetMathLibrary.BreakRotator` (`KismetMathLibrary.FindLookAtRotation` (`self.K2_GetActorLocation`) (`self.K2_GetActorLocation` (`self.AttackTarget`)))))
  ;[1 0.8386 0] Track Player
  (`self.AttackTarget`
    (:`then`
      (if (`self.AttackingPlayer?`)
        (`self.K2_SetActorRotation` (`KismetMathLibrary.MakeRotator` 0.0 0.0 _returnvalue_yaw))
        (`KismetSystemLibrary.Delay` 0.01)
        (`self.TrackPlayer`)))
    (:`else`)))

(event `self.ShowHealthBar.OnComponentBeginOverlap`
  (params (OverlappedComponent :type "PrimitiveComponent Object Reference") (OtherActor :type "Actor Object Reference") (OtherComp :type "PrimitiveComponent Object Reference") (OtherBodyIndex :type Integer) (bFromSweep :type Boolean) (SweepResult :type "HitResult Structure (by ref)"))
  ;[0.07721 0 1] Display enemy health bar
  (cast `/Game/FlexibleCombatSystem/Blueprints/BP_PlayerCharacter` OtherActor)
  (`SceneComponent.SetVisibility` (`self.HealthBar`) true false))

(event `SetDamage`
  ;[1 0 0.0148] Apply Damage
  (bind _output_get (set `self.Health` (- (`self.Health`) 10.0)))
  (set `/Game/ProjectHooks/Blueprints/Mutant/WBP_HealthBarEnemy.Health` _output_get (`self.HealthWidgetRef`))
  (if (<= (`self.Health`) 0.0)
    (set `self.Dead?` true)
    (`KismetSystemLibrary.Delay` 10.0)
    (`self.K2_DestroyActor` self)
    (bind _asbp_game_modee (cast `/Game/FlexibleCombatSystem/Blueprints/BP_GameModee` (`GameplayStatics.GetGameMode`)))
    (`/Game/FlexibleCombatSystem/Blueprints/BP_GameModee.SaveGame` _asbp_game_modee)))

(event `self.ShowHealthBar.OnComponentEndOverlap`
  (params (OverlappedComponent :type "PrimitiveComponent Object Reference") (OtherActor :type "Actor Object Reference") (OtherComp :type "PrimitiveComponent Object Reference") (OtherBodyIndex :type Integer))
  ;[0.07721 0 1] Display enemy health bar
  (cast `/Game/FlexibleCombatSystem/Blueprints/BP_PlayerCharacter` OtherActor)
  (`SceneComponent.SetVisibility` (`self.HealthBar`) false false))

(fn `AttackTrace`
  (bind _returnvalue (`self.K2_GetActorLocation`))
  (bind _attackdamage (`self.AttackDamage`))
  (bind (_outhit _returnvalue_2) (`KismetSystemLibrary.SphereTraceSingle` :`Start` _returnvalue :`End` (+ _returnvalue (* (`self.GetActorForwardVector`) (`self.AttackRange`))) :`Radius` (`self.AttackRadius`) :`TraceChannel` "TraceTypeQuery1" :`DrawDebugType` "ForDuration"))
  (if _returnvalue_2
    (`GameplayStatics.ApplyDamage` (`.HitActor` (`GameplayStatics.BreakHitResult` _outhit)) (`KismetMathLibrary.Conv_IntToDouble` (`KismetMathLibrary.Round` (`KismetMathLibrary.RandomFloatInRange` (- _attackdamage 2.0) (+ _attackdamage 2.0)))))))

(fn `UpdatePatrolPoint`
  (bind _outactors (`GameplayStatics.GetAllActorsOfClass` "/Game/ProjectHooks/Blueprints/Mutant/BP_EnemyPatrolPoint.BP_EnemyPatrolPoint_C"))
  (for _array_element _outactors
    (if (< (`self.GetDistanceTo` _array_element self) (`self.GetDistanceTo` (`self.PatrolPointRef`) self))
      (set `self.PatrolPointRef` _array_element))))

(fn `UserConstructionScript`
  (bind _outactors (`GameplayStatics.GetAllActorsOfClass` "/Game/ProjectHooks/Blueprints/Mutant/BP_EnemyPatrolPoint.BP_EnemyPatrolPoint_C"))
  (set `self.PatrolPointRef` (`|GetArrayItem` _outactors))
  (for _array_element _outactors
    (if (< (`self.GetDistanceTo` _array_element self) (`self.GetDistanceTo` (`self.PatrolPointRef`) self))
      (set `self.PatrolPointRef` _array_element))))