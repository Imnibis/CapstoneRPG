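; B_Health is a health component that tracks damage, healing and death for its owning actor.
; On BeginPlay it binds to the owner's TakeAnyDamage event, subtracting clamped damage unless the owner is dead or within a real-time invulnerability window after the last hit.
; ApplyHeal restores health up to the maximum while alive.
; OnHeal, OnDamage and OnDeath events broadcast the results, with death firing before the final damage event.
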(event `ApplyHeal`
  (params (Amount :type "Float (double-precision)"))
  ;[1 1 1] HealingSystem
  (if (and (not (`self.isDead`)) (!= (`self.Health`) (`self.MaxHealth`)))
    (bind _output_get (set `self.Health` (`KismetMathLibrary.FClamp` (+ (`self.Health`) Amount) 0.0 (`self.MaxHealth`))))
    (`self.Event OnHeal` Amount _output_get)))

(event `OnTakeAnyDamage`
  (params (DamagedActor :type "Actor Object Reference") (Damage :type "Float (single-precision)") (DamageType :type "DamageType Object Reference") (InstigatedBy :type "Controller Object Reference") (DamageCauser :type "Actor Object Reference"))
  ;[1 1 1] DamageSystem
  (if (and (not (`self.isDead`)) (> (- (`GameplayStatics.GetRealTimeSeconds`) (`self.LastDamageTime`)) (`self.InvulnerabilityDuration`)))
    (bind _output_get (set `self.Health` (`KismetMathLibrary.FClamp` (- (`self.Health`) Damage) 0.0 (`self.MaxHealth`))))
    (set `self.LastDamageTime` (`GameplayStatics.GetRealTimeSeconds`))
    (if (<= _output_get 0.0)
      (`self.Event OnDeath` DamagedActor Damage DamageType InstigatedBy DamageCauser)
      (set `self.isDead` true))
    (`self.Event OnDamage` DamagedActor Damage DamageType InstigatedBy DamageCauser (`self.Health`))))

(event `self.ReceiveBeginPlay`
  ;[1 1 1] BeginPlay
  (add `Actor.OnTakeAnyDamage` (`self.GetOwner`) (delegate `OnTakeAnyDamage`)))