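; B_Targetable is a component that shows a screen-space target indicator on its owning actor.
; On BeginPlay it adds a WidgetComponent to the owner and sets it to Screen space.
; OnTarget creates a TargetIndicatorWidget and assigns it to that component, while OnUntarget destroys the widget and clears the reference.
; Both targeting events also print debug strings.
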(event `self.ReceiveBeginPlay`
  (bind _returnvalue (`|AddComponentByClass` :`self` (`self.GetOwner`) :`Class` "/Script/UMG.WidgetComponent"))
  (bind _output_get (set `self.WidgetComponent` _returnvalue))
  (`WidgetComponent.SetWidgetSpace` _output_get "Screen"))

(event `OnTarget`
  (`KismetSystemLibrary.PrintString` "Targeted")
  (bind _returnvalue (`|CreateWidget` "/Game/ProjectHooks/Widgets/TargetIndicatorWidget.TargetIndicatorWidget_C"))
  (bind _output_get (set `self.Widget` _returnvalue))
  (`WidgetComponent.SetWidget` (`self.WidgetComponent`) _output_get))

(event `OnUntarget`
  (`KismetSystemLibrary.PrintString` "Untargeted")
  (`/Game/ProjectHooks/Widgets/TargetIndicatorWidget.Destroy` (`self.Widget`))
  (set `self.Widget` null))