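; Spline layout tool actor that places copies of a chosen mesh along a spline as instanced static meshes.
; Construction script rebuilds the instances, spacing them by the mesh's X bounds plus an offset and aiming each at the next position.
; Optional alternating rotation switches even-indexed instances' up reference from Z to Y, like chain links.
; SetSplinePointsAndUpdate lets callers replace the spline points and rebuild the layout.
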(fn `GetLocationAtIndex`
  (params (Index :type Integer))
  (returns (Location :type "Vector Structure"))
  (return (`SplineComponent.GetLocationAtDistanceAlongSpline` (`self.Spline`) (* Index (`self.Spacing`)) "Local")))

(fn `SetSplinePointsAndUpdate`
  (params (Points :type "Array of Vector Structure (by ref)") (CoordinateSpace :type "ESplineCoordinateSpace Enum" :default "Local") (bUpdateSpline :type Boolean))
  (`SplineComponent.SetSplinePoints` (`self.Spline`) Points CoordinateSpace bUpdateSpline)
  (`self.UpdateMeshes`))

(fn `UpdateMeshes`
  (locals (NumberOfInstances :type Integer))
  (bind _instancedstaticmesh (`self.InstancedStaticMesh`))
  (bind (_returnvalue_min _returnvalue_max) (break `Box` (`StaticMesh.GetBoundingBox` (`self.PlacedMesh`))))
  (bind _returnvalue_x (`KismetMathLibrary.BreakVector` (- _returnvalue_max _returnvalue_min)))
  (`InstancedStaticMeshComponent.ClearInstances` _instancedstaticmesh)
  (`StaticMeshComponent.SetStaticMesh` _instancedstaticmesh (`self.PlacedMesh`))
  (bind _output_get (set `self.Spacing` (+ _returnvalue_x (`self.Offset`))))
  (bind _output_get_2 (set `local.NumberOfInstances` (`KismetMathLibrary.FFloor` (/ (`SplineComponent.GetSplineLength` (`self.Spline`)) _output_get))))
  (for _index (range (+ _output_get_2 1))
    (bind _location (`self.GetLocationAtIndex` _index))
    (`InstancedStaticMeshComponent.AddInstance` (`self.InstancedStaticMesh`) (`KismetMathLibrary.MakeTransform` _location (`KismetMathLibrary.MakeRotFromXZ` (- (`self.GetLocationAtIndex` (+ _index 1)) _location) (`KismetMathLibrary.SelectVector` (0.0 1.0 0.0) (0.0 0.0 1.0) (and (== (mod _index 2) 0) (`self.AlternateRotations`))))) false)))

(fn `UserConstructionScript`
  (`self.UpdateMeshes`))